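; BP_Triggerable is a trigger actor that reacts when Characters enter or leave its Trigger component.
; Both component overlap events pass the other actor through ShouldTriggerReactToActor, which accepts only Character and its subclasses.
; Accepted actors are forwarded to separate Overlap and Unoverlap events, which currently just print the actor's display name.
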(event OnComponentBeginOverlap(Trigger)
  (params (OverlappedComponent :type Primitive%20Component%20Object%20Reference) (OtherActor :type Actor%20Object%20Reference) (OtherComp :type Primitive%20Component%20Object%20Reference) (OtherBodyIndex :type Integer) (bFromSweep :type Boolean) (SweepResult :type Hit%20Result%20Structure%20%28by%20ref%29))
  (bind _shouldreact (CallFunction|ShouldTriggerReacttoActor OtherActor))
  (if _shouldreact
    (CallFunction|Overlap OtherActor)))

(event OnComponentEndOverlap(Trigger)
  (params (OverlappedComponent :type Primitive%20Component%20Object%20Reference) (OtherActor :type Actor%20Object%20Reference) (OtherComp :type Primitive%20Component%20Object%20Reference) (OtherBodyIndex :type Integer))
  (bind _shouldreact (CallFunction|ShouldTriggerReacttoActor OtherActor))
  (if _shouldreact
    (CallFunction|Unoverlap OtherActor)))

(event Custom|Overlap
  (params (Other%20Actor :type Actor%20Object%20Reference))
  (Development|PrintString (Utilities|GetDisplayName Other%20Actor)))

(event Custom|Unoverlap
  (params (Other%20Actor :type Actor%20Object%20Reference))
  (Development|PrintString (Utilities|GetDisplayName Other%20Actor)))

(event EventBeginPlay)

(event Collision|EventActorBeginOverlap
  (params (OtherActor :type Actor%20Object%20Reference)))

(event EventTick
  (params (DeltaSeconds :type Float%20%28single-precision%29)))

(fn ConstructionScript)

(fn ShouldTriggerReacttoActor
  (params (ActorToCheck :type Actor%20Object%20Reference))
  (return (Utilities|ClassIsChildOf (Utilities|GetClass ActorToCheck) "/Script/Engine.Character")))